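; Wall Blueprint actor that registers itself with the player's MrGear pawn while the two overlap.
; On begin overlap with player pawn 0, it casts to MrGear, passes itself to RememberWall and calls StopFlying.
; On end overlap it calls ForgetWall with itself, leaving the wall tracking to MrGear.
; The construction script only calls its parent.
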(event `self.ReceiveActorBeginOverlap`
  (params (OtherActor :type "Actor Object Reference"))
  (bind _returnvalue (`GameplayStatics.GetPlayerPawn` 0))
  (if (== OtherActor _returnvalue)
    (bind _asmr_gear (cast `/Game/MyContent/Blueprints/MrGear` _returnvalue))
    (`/Game/MyContent/Blueprints/MrGear.RememberWall` _asmr_gear self)
    (`/Game/MyContent/Blueprints/MrGear.StopFlying` _asmr_gear)))

(event `self.ReceiveActorEndOverlap`
  (params (OtherActor :type "Actor Object Reference"))
  (bind _returnvalue (`GameplayStatics.GetPlayerPawn` 0))
  (if (== OtherActor _returnvalue)
    (bind _asmr_gear (cast `/Game/MyContent/Blueprints/MrGear` _returnvalue))
    (`/Game/MyContent/Blueprints/MrGear.ForgetWall` _asmr_gear self)))

(fn `UserConstructionScript`
  (`parent.UserConstructionScript`))