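; Player pawn that moves along its right and up axes while its camera rolls around a center point.
; Two input axes add movement input scaled by MaxSpeed, which Tick consumes and applies as a frame-time-scaled local offset without sweeping.
; Each Tick also sets the camera's world roll from the atan2 angle of the center-to-player direction in the YZ plane, keeping screen-up pointing away from CenterLocation.
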(event `InputAxis|MoveHorizontally`
  (params (AxisValue :type "Float (single-precision)"))
  ;[1 1 1] Horizontal moving
  (`self.AddMovementInput` (`self.GetActorRightVector`) (* AxisValue (`self.MaxSpeed`))))

(event `InputAxis|MoveVertically`
  (params (AxisValue :type "Float (single-precision)"))
  ;[1 1 1] Vertical Moving
  (`self.AddMovementInput` (`self.GetActorUpVector`) (* AxisValue (`self.MaxSpeed`))))

(event `self.ReceiveTick`
  (params (DeltaSeconds :type "Float (single-precision)"))
  (bind (_returnvalue_x _returnvalue_y _returnvalue_z) (`KismetMathLibrary.BreakVector` (`KismetMathLibrary.GetDirectionUnitVector` (`self.CenterLocation`) (`self.K2_GetActorLocation`))))
  ;[1 1 1] Moving
  (bind _returnvalue (`self.ConsumeMovementInputVector`))
  (`self.K2_AddActorLocalOffset` (* _returnvalue DeltaSeconds))
  ;[1 1 1] Camera Rotating
  (`SceneComponent.K2_SetWorldRotation` (`self.Camera`) (`KismetMathLibrary.MakeRotator` (+ (* (`KismetMathLibrary.DegAtan2` _returnvalue_z _returnvalue_y) -1.0) 90.0)) false false))

(fn `UserConstructionScript`)