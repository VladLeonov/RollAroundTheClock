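; Center actor that endlessly builds a radial level of Wall and Spike blocks closing in on its position.
; BeginPlay sizes the rings and stacks level parts outward to CreationDistance, spawning each matrix row as a ring around the X axis.
; Tick steps blocks inward, rescales their Z by radius to fit the shrinking ring, and destroys them inside DestroyingDistance.
; When the tracked outer edge reaches CreationDistance, it appends a part generated from the previous one.
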(event `self.ReceiveBeginPlay`
  ;[1 1 1] Initializing Section
  (`self.CalculateNumBlockInRing`)
  (`self.CalculateAngleDelta`)
  (`self.CalculateLastLevelPartDistance`)
  ;[1 1 1] First Build Section
  (`self.CalculateFirstLevelPart`)
  (`self.BuildLastLevelPart` :!label _label)
  (if (<= (`self.LastLevelPartDistance`) (`self.CreationDistance`))
    (goto _label)))

(event `self.ReceiveTick`
  (params (DeltaSeconds :type "Float (single-precision)"))
  ;[1 1 1] Blocks Updating Section
  (for (_array_element _array_index) (`self.Block Array`)
    (bind _isblockdestroyed (`self.DestroyBlockIfNeeded` _array_element _array_index))
    (if (not _isblockdestroyed)
      (`self.MoveBlockToCenter` _array_element)
      (`self.ScaleBlock` _array_element)))
  ;[1 1 1] Building Level Parts Section
  (bind _needtobuildnextlevelpart (`self.UpdateLastLevelPartDistance`))
  (if _needtobuildnextlevelpart
    (`self.BuildNextLevelPart`)))

(fn `BuildLastLevelPart`
  (bind (_arrayindex _arrayelement) (`/Engine/EditorBlueprintResources/StandardMacros.ReverseForEachLoop` (`.blockMatrix` (break `LevelPart` (`self.LastLevelPart`))))
    (:`LoopBody`
      (set `self.Angle` 0.0)
      (for _array_element (`.elements` (break `BlockArray` _arrayelement))
        (bind (_blocktype _direction) (break `DirectionalBlock` _array_element))
        (bind _actor_type (`self.GetActorTypeFormBlockType` _blocktype))
        (if (not (== _actor_type null))
          (`self.CreateBlock` _actor_type _direction (`self.LastLevelPartDistance`)))
        (`self.UpdateAngle`))
      (`self.IncreaseLastLevelPartDistance`))))

(fn `BuildNextLevelPart`
  (bind _returnvalue (`LevelGenerator.createNextLevelPart` (`self.LastLevelPart`)))
  (set `self.LastLevelPart` _returnvalue)
  (`self.BuildLastLevelPart`))

(fn `CalculateAngleDelta`
  (set `self.AngleDelta` (/ 360.0 (`KismetMathLibrary.Conv_IntToDouble` (`self.NumBlocksInWidth`)))))

(fn `CalculateFirstLevelPart`
  (bind _returnvalue (`LevelGenerator.createFirstLevelPart` (`self.NumBlocksInWidth`) (`self.NumBlockInHeight`)))
  (set `self.LastLevelPart` _returnvalue))

(fn `CalculateLastLevelPartDistance`
  (set `self.LastLevelPartDistance` (+ (`self.DestroyingDistance`) (`self.BlockSize`))))

(fn `CalculateNumBlockInRing`
  (set `self.NumBlocksInWidth` (`KismetMathLibrary.Round` (/ (* (+ (`self.CreationDistance`) (`self.DestroyingDistance`)) (`KismetMathLibrary.GetPI`)) (`self.BlockSize`)))))

(fn `CreateBlock`
  (params (ClassType :type "Actor Class Reference") (Direction :type "EDirection Enum" :default "UP") (DistanceToCenter :type "Float (double-precision)"))
  (bind _returnvalue (`KismetMathLibrary.MakeRotator` (`self.Angle`)))
  (bind _angle (`self.GetAngleFromDirection` Direction))
  (bind _returnvalue_2 (`|SpawnActorFromClass` ClassType (`KismetMathLibrary.MakeTransform` (+ (`SceneComponent.K2_GetComponentLocation` (`self.Root`)) (`KismetMathLibrary.GreaterGreater_VectorRotator` (`KismetMathLibrary.MakeVector` 0.0 DistanceToCenter) _returnvalue)) (`KismetMathLibrary.ComposeRotators` _returnvalue (`KismetMathLibrary.MakeRotator` _angle)) (`KismetMathLibrary.MakeVector` 1.0 1.0 (/ (* DistanceToCenter 2.0) (+ (`self.CreationDistance`) (`self.DestroyingDistance`))))) "Undefined" "OverrideRootScale" null null))
  (bind _asblock (cast `/Game/MyContent/Blueprints/Block` _returnvalue_2))
  (`KismetArrayLibrary.Array_Add` (`self.Block Array`) _asblock))

(fn `DestroyBlockIfNeeded`
  (params (Block :type "/Game/MyContent/Blueprints/Block Object Reference") (ArrayIndex :type Integer))
  (returns (IsBlockDestroyed :type Boolean))
  (bind _returnvalue (< (`self.GetDistanceTo` Block) (`self.DestroyingDistance`)))
  (if _returnvalue
    (`self.K2_DestroyActor` Block)
    (`KismetArrayLibrary.Array_Remove` (`self.Block Array`) ArrayIndex))
  (return _returnvalue))

(fn `GetActorTypeFormBlockType`
  (params (`Block Type` :type "EBlockType Enum" :default "EMPTY"))
  (returns (`Actor type` :type "Actor Class Reference"))
  (switch `EBlockType` `Block Type`
    (:`EMPTY`
      (return null))
    (:`WALL`
      (return "/Game/MyContent/Blueprints/Wall.Wall_C"))
    (:`SPIKE`
      (return "/Game/MyContent/Blueprints/Spike.Spike_C"))))

(fn `GetAngleFromDirection`
  (params (Direction :type "EDirection Enum" :default "UP"))
  (returns (Angle :type "Float (double-precision)"))
  (switch `EDirection` Direction
    (:`UP`
      (return 0.0))
    (:`RIGHT`
      (return 90.0))
    (:`DOWN`
      (return 180.0))
    (:`LEFT`
      (return 270.0))))

(fn `IncreaseLastLevelPartDistance`
  (set `self.LastLevelPartDistance` (+ (`self.LastLevelPartDistance`) (`self.BlockSize`))))

(fn `MoveBlockToCenter`
  (params (Block :type "/Game/MyContent/Blueprints/Block Object Reference"))
  (bind _returnvalue (`self.K2_GetActorLocation` Block))
  (`self.K2_SetActorLocation` Block (+ _returnvalue (* (`KismetMathLibrary.GetDirectionUnitVector` _returnvalue (`SceneComponent.K2_GetComponentLocation` (`self.Root`))) (`self.MovingStep`))) false false))

(fn `ScaleBlock`
  (params (Block :type "/Game/MyContent/Blueprints/Block Object Reference"))
  (`self.SetActorScale3D` Block (`KismetMathLibrary.MakeVector` 1.0 1.0 (/ (`KismetMathLibrary.VSize` (- (`self.K2_GetActorLocation` Block) (`SceneComponent.K2_GetComponentLocation` (`self.Root`)))) (/ (- (+ (`self.CreationDistance`) (`self.DestroyingDistance`)) (`self.BlockSize`)) 2.0)))))

(fn `UpdateAngle`
  (set `self.Angle` (+ (`self.Angle`) (`self.AngleDelta`))))

(fn `UpdateLastLevelPartDistance`
  (returns (NeedToBuildNextLevelPart :type Boolean))
  (set `self.LastLevelPartDistance` (- (`self.LastLevelPartDistance`) (`self.MovingStep`)))
  (return (<= (`self.LastLevelPartDistance`) (`self.CreationDistance`))))

(fn `UserConstructionScript`)